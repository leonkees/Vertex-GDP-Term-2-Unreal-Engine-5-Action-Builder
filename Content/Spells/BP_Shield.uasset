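; Shield spell actor that attaches itself to the player character and lasts five seconds.
; On BeginPlay it snaps to the pelvis socket of the BP_TopDownCharacter mesh, keeping world scale, then destroys itself after a delay.
; It calls IgnoreActorWhenMoving on its sphere collision without specifying an actor.
; Overlap and Tick events are empty, and an older socket-following teleport is left disconnected.
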(event EventBeginPlay
  (bind _asbp_top_down_character (Utilities|Casting|CastToBP_TopDownCharacter (Game|GetPlayerCharacter 0)))
  (Transformation|AttachComponentToComponent (Variables|/Script/Engine.Character|GetMesh _asbp_top_down_character) "pelvis" "SnapToTarget" "SnapToTarget" "KeepWorld" true)
  (Collision|IgnoreActorwhenMoving (Variables|Default|GetSphereCollision) 0 true)
  (Utilities|FlowControl|Delay 5.0)
  (Actor|DestroyActor))

(event Collision|EventActorBeginOverlap
  (params (OtherActor :type Actor%20Object%20Reference)))

(event EventTick
  (params (DeltaSeconds :type Float%20%28single-precision%29)))

(fn ConstructionScript)