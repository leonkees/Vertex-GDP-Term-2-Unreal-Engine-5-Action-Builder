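; BP_CardPickup is a world pickup that opens the spell pickup screen when the player character touches it.
; On mesh overlap with the player it destroys itself, shows WBP_SpellPIckupScreen, sets Game and UI input and pauses the game.
; Disconnected leftover nodes would add a random DT_AllCards spell to the character's FullDeck, but they never run.
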(event OnComponentBeginOverlap(StaticMesh)
  (params (OverlappedComponent :type Primitive%20Component%20Object%20Reference) (OtherActor :type Actor%20Object%20Reference) (OtherComp :type Primitive%20Component%20Object%20Reference) (OtherBodyIndex :type Integer) (bFromSweep :type Boolean) (SweepResult :type Hit%20Result%20Structure%20%28by%20ref%29))
  (if (== OtherActor (Game|GetPlayerCharacter 0))
    (Actor|DestroyActor)
    (bind _returnvalue (UserInterface|CreateWidget "/Game/TopDown/Blueprints/SpellPickupWBP/WBP_SpellPIckupScreen.WBP_SpellPIckupScreen_C"))
    (UserInterface|Viewport|AddtoViewport _returnvalue 0)
    (Input|SetInputModeGameandUI (Game|GetPlayerController 0) _returnvalue "DoNotLock" true false)
    (Class|WidgetBlueprintLibrary|SetFocustoGameViewport)
    (Game|SetGamePaused true)))

(event EventBeginPlay)

(event Collision|EventActorBeginOverlap
  (params (OtherActor :type Actor%20Object%20Reference)))

(event EventTick
  (params (DeltaSeconds :type Float%20%28single-precision%29)))

(fn ConstructionScript)