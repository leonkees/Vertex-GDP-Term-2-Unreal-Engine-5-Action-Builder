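; BP_Ice is a short-lived ice spell actor that applies a freezing effect to enemies it touches.
; On BeginPlay it attaches to the player character's pelvis socket, then destroys itself two seconds later.
; Capsule overlaps with Enemy-tagged actors implementing BPI_EffectSystem send an ApplyEffect message with a blue tint, a timed duration and zero speed factor.
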(event OnComponentBeginOverlap(Capsule)
  (params (OverlappedComponent :type Primitive%20Component%20Object%20Reference) (OtherActor :type Actor%20Object%20Reference) (OtherComp :type Primitive%20Component%20Object%20Reference) (OtherBodyIndex :type Integer) (bFromSweep :type Boolean) (SweepResult :type Hit%20Result%20Structure%20%28by%20ref%29))
  (if (Actor|ActorHasTag OtherActor "Enemy")
    (if (Utilities|DoesObjectImplementInterface OtherActor "/Game/Enemies/BPI_EffectSystem.BPI_EffectSystem_C")
      (Class|BPIEffectSystem|ApplyEffect(Message) OtherActor "0.300000,0.300000,1.000000" 1e+01 0.0))))

(event Collision|EventActorBeginOverlap
  (params (OtherActor :type Actor%20Object%20Reference)))

(event EventTick
  (params (DeltaSeconds :type Float%20%28single-precision%29)))

(event EventBeginPlay
  (bind _asbp_top_down_character (Utilities|Casting|CastToBP_TopDownCharacter (Game|GetPlayerCharacter 0)))
  (Transformation|AttachComponentToComponent (Variables|/Script/Engine.Character|GetMesh _asbp_top_down_character) "pelvis" "SnapToTarget" "SnapToTarget" "KeepRelative" true)
  (Utilities|FlowControl|Delay 2.0)
  (Actor|DestroyActor))

(fn ConstructionScript)