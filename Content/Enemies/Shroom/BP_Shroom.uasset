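; BP_Shroom is an enemy that damages BP_TopDownCharacter through an attack collider switched on and off by enable and disable events.
; Incoming damage goes to the ACStats component, whose health update event destroys the actor once health reaches zero or below.
; ApplyEffect temporarily scales walk speed and tints the mesh, then after a delay restores a white tint and a hard-coded walk speed.
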(event OnComponentBeginOverlap(AttackCollider)
  (params (OverlappedComponent :type Primitive%20Component%20Object%20Reference) (OtherActor :type Actor%20Object%20Reference) (OtherComp :type Primitive%20Component%20Object%20Reference) (OtherBodyIndex :type Integer) (bFromSweep :type Boolean) (SweepResult :type Hit%20Result%20Structure%20%28by%20ref%29))
  (if (not (== OtherActor self))
    (Utilities|Casting|CastToBP_TopDownCharacter OtherActor)
    (if (Variables|Default|GetHitEnable)
      (Game|Damage|ApplyDamage OtherActor 1.0 0 0))))

(event Custom|OnHealthUpdated_Event
  (params (UpdatedHealth :type Integer))
  (if (not (> UpdatedHealth 0))
    (Actor|DestroyActor)))

(event Custom|EnableAttackCollider
  ;[0.15 0.15 0.15 0.5] Attack Collider Enable/Disable
  (Collision|SetCollisionEnabled (Variables|Default|GetAttackCollider) "QueryOnly")
  (Variables|Default|SetHitEnable true))

(event Custom|DisableAttackCollider
  ;[0.15 0.15 0.15 0.5] Attack Collider Enable/Disable
  (Collision|SetCollisionEnabled (Variables|Default|GetAttackCollider) "NoCollision")
  (Variables|Default|SetHitEnable false))

(event EventBeginPlay
  (EventDispatchers|AssignOnHealthUpdated (Variables|Default|GetAC_Stats) (delegate Custom|OnHealthUpdated_Event)))

(event Collision|EventActorBeginOverlap
  (params (OtherActor :type Actor%20Object%20Reference)))

(event EventTick
  (params (DeltaSeconds :type Float%20%28single-precision%29)))

(event Game|Damage|EventAnyDamage
  (params (Damage :type Float%20%28single-precision%29) (DamageType :type Damage%20Type%20Object%20Reference) (InstigatedBy :type Controller%20Object%20Reference) (DamageCauser :type Actor%20Object%20Reference))
  (Default|UpdateHealth (Variables|Default|GetAC_Stats) (Math|Float|Truncate (* Damage -1.0))))

(event EventApplyEffect
  (params (Color :type Vector :default "0, 0, 0") (Time :type Float%20%28double-precision%29) (SpeedFactor :type Float%20%28double-precision%29))
  (bind _charactermovement (Variables|Character|GetCharacterMovement))
  (bind _output_get (Variables|Default|SetSpeedFactor SpeedFactor))
  (Variables|/Script/Engine.CharacterMovementComponent|SetMaxWalkSpeed _charactermovement (* _output_get (Class|MovementComponent|GetMaxSpeed _charactermovement)))
  (Rendering|Material|SetColorParameterValueonMaterials (Variables|Character|GetMesh) "EffectTint" (Math|Conversions|ToLinearColor(Vector) Color))
  (Utilities|FlowControl|Delay Time)
  (Variables|Default|SetSpeedFactor 1.0)
  (Rendering|Material|SetColorParameterValueonMaterials (Variables|Character|GetMesh) "EffectTint" (Math|Color|MakeColor 1.0 1.0 1.0))
  (Variables|/Script/Engine.CharacterMovementComponent|SetMaxWalkSpeed _charactermovement 6e+02))

(fn ConstructionScript)